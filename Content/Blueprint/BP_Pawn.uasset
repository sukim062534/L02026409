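; BP_Pawn is a player-controlled flying pawn that constantly moves along its forward vector each tick through FloatingPawnMovement.
; Roll and Pitch axes rotate it locally at a frame-rate-independent rate, so steering changes the flight direction.
; Holding Boost raises max speed and acceleration while lowering deceleration, restoring them on release.
; Fire spawns BP_Fire at the Arrow component's transform and prints a debug string.
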(event EventTick
  (params (DeltaSeconds :type Float%20%28single-precision%29))
  ;[0.15 0.15 0.15 0.5] 앞으로 이동
  (Pawn|Input|AddMovementInput (Transformation|GetActorForwardVector) 1.0 false))

(event Input|ActionEvents|InputActionFire
  (params (Key :type Key%20Structure :default "None"))
  (:Pressed
    (Game|SpawnActorfromClass "/Game/Blueprint/BP_Fire.BP_Fire_C" (Transformation|GetWorldTransform (Variables|Default|GetArrow)) "AdjustIfPossibleButDontSpawnIfColliding" "MultiplyWithRoot" 0 0)
    (Development|PrintString "Hello")))

(event Input|ActionEvents|InputActionBoost
  (params (Key :type Key%20Structure :default "None"))
  (bind _floatingpawnmovement (Variables|Default|GetFloatingPawnMovement))
  (bind _floatingpawnmovement_2 (Variables|Default|GetFloatingPawnMovement))
  (:Pressed
    (Variables|/Script/Engine.FloatingPawnMovement|SetMaxSpeed _floatingpawnmovement_2 1.2e+03)
    (Variables|/Script/Engine.FloatingPawnMovement|SetAcceleration _floatingpawnmovement_2 6e+03)
    (Variables|/Script/Engine.FloatingPawnMovement|SetDeceleration _floatingpawnmovement_2 8e+02))
  (:Released
    (Variables|/Script/Engine.FloatingPawnMovement|SetMaxSpeed _floatingpawnmovement 5e+02)
    (Variables|/Script/Engine.FloatingPawnMovement|SetAcceleration _floatingpawnmovement 2e+03)
    (Variables|/Script/Engine.FloatingPawnMovement|SetDeceleration _floatingpawnmovement 3e+03)))

(event Input|AxisEvents|InputAxisRoll
  (params (AxisValue :type Float%20%28single-precision%29))
  ;[0.15 0.15 0.15 0.5] Roll
  (Transformation|AddActorLocalRotation (Math|Rotator|MakeRotator (* AxisValue 6e+01 (Utilities|Time|GetWorldDeltaSeconds)) 0.0 0.0) false false))

(event Input|AxisEvents|InputAxisPitch
  (params (AxisValue :type Float%20%28single-precision%29))
  ;[0.15 0.15 0.15 0.5] Pitch
  (Transformation|AddActorLocalRotation (Math|Rotator|MakeRotator 0.0 (* AxisValue 6e+01 (Utilities|Time|GetWorldDeltaSeconds)) 0.0) false false))

(fn ConstructionScript)